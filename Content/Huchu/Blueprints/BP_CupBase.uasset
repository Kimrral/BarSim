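; BP_CupBase is a base cup Blueprint that detects bar spoon stirring and plays glass clinks.
; Spoon overlaps with two sphere triggers raise the stir rate, reset its timer and toggle StirStarted, provided the cup is at least a tenth full.
; Hits against other cups spawn a randomly pitched clank at the impact point, gated by DoOnce, a short delay and audio component checks to limit repeats.
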(event OnComponentBeginOverlap(Sphere1)
  (params (OverlappedComponent :type Primitive%20Component%20Object%20Reference) (OtherActor :type Actor%20Object%20Reference) (OtherComp :type Primitive%20Component%20Object%20Reference) (OtherBodyIndex :type Integer) (bFromSweep :type Boolean) (SweepResult :type Hit%20Result%20Structure%20%28by%20ref%29))
  (Utilities|Casting|CastToBarSpoon OtherActor)
  (if (>= (/ (Variables|Default|Getcontents) (Variables|Default|GetcupSize)) 0.1)
    (Utilities|FlowControl|FlipFlop
      (:A
        (Variables|Default|SetbStirStarted true))
      (:B
        (Variables|Default|SetbStirStarted false)))
    (Variables|Default|SetstirRate (+ (Variables|Default|GetstirRate) 0.5))
    (Variables|Default|SettimePassed 0.0)))

(event OnComponentBeginOverlap(Sphere)
  (params (OverlappedComponent :type Primitive%20Component%20Object%20Reference) (OtherActor :type Actor%20Object%20Reference) (OtherComp :type Primitive%20Component%20Object%20Reference) (OtherBodyIndex :type Integer) (bFromSweep :type Boolean) (SweepResult :type Hit%20Result%20Structure%20%28by%20ref%29))
  (Utilities|Casting|CastToBarSpoon OtherActor)
  (if (>= (/ (Variables|Default|Getcontents) (Variables|Default|GetcupSize)) 0.1)
    (Utilities|FlowControl|FlipFlop
      (:A
        (Variables|Default|SetbStirStarted true))
      (:B
        (Variables|Default|SetbStirStarted false)))
    (Variables|Default|SetstirRate (+ (Variables|Default|GetstirRate) 0.5))
    (Variables|Default|SettimePassed 0.0)))

(event OnComponentHit(cupComp)
  (params (HitComponent :type Primitive%20Component%20Object%20Reference) (OtherActor :type Actor%20Object%20Reference) (OtherComp :type Primitive%20Component%20Object%20Reference) (NormalImpulse :type Vector :default "0, 0, 0") (Hit :type Hit%20Result%20Structure%20%28by%20ref%29))
  (bind _ascup_base (Utilities|Casting|CastToCupBase OtherActor))
  (Utilities|IsValid (Variables|/Script/BarSim.CupBase|GetglassClankAudioComp _ascup_base)
    (:Is%20Valid
      (Utilities|FlowControl|DoOnce false
        (:Completed
          (if (not (Audio|Components|Audio|IsPlaying (Variables|/Script/BarSim.CupBase|GetglassClankAudioComp _ascup_base)))
            (bind _returnvalue (Audio|SpawnSoundatLocation "/Game/KHJContents/Sounds/BottleClank/GlassClank.GlassClank" (.Location (Collision|BreakHitResult Hit)) "0, 0, 0" 0.5 (Math|Random|RandomFloatinRange 1.6 1.7) 0.0 0 0 :!label _label))
            (Variables|Default|SetglassClankAudioComp _returnvalue)
            (Utilities|FlowControl|Delay 0.2)
            (goto _label_2 Reset)))))
    (:Is%20Not%20Valid
      (Utilities|FlowControl|DoOnce false :!label _label_2
        (:Completed
          (goto _label))))))

(event Collision|EventActorBeginOverlap
  (params (OtherActor :type Actor%20Object%20Reference)))

(event EventTick
  (params (DeltaSeconds :type Float%20%28single-precision%29)))

(fn ConstructionScript)